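; Game mode that tracks the player's score and shows the game over screen.
; BeginPlay adds the WB_Score widget to the viewport.
; TambahScore increments and prints PlayerScore, then calls Kalah when the score reaches one.
; Kalah displays WB_GameOver and enables the mouse cursor; unconnected leftover nodes for input modes and a GameOver flag never run.
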(event `self.ReceiveBeginPlay`
  (bind _returnvalue (`|CreateWidget` "/Game/BluePrint/FallingObject/WB_Score.WB_Score_C"))
  (`UserWidget.AddToViewport` _returnvalue 0))

(fn `Kalah`
  (bind _returnvalue (`|CreateWidget` "/Game/BluePrint/FallingObject/WB_GameOver.WB_GameOver_C"))
  (`UserWidget.AddToViewport` _returnvalue 0)
  (set `PlayerController.bShowMouseCursor` true (`GameplayStatics.GetPlayerController` 0)))

(fn `TambahScore`
  (set `self.PlayerScore` (+ (`self.PlayerScore`) 1))
  (`KismetSystemLibrary.PrintString` (`KismetStringLibrary.Conv_IntToString` (`self.PlayerScore`)))
  (if (== (`self.PlayerScore`) 1)
    (`self.Kalah`)))

(fn `UserConstructionScript`)